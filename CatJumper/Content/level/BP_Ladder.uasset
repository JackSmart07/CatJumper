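; BP_Ladder is a ladder actor that lets BP_Player climb while inside its Box trigger.
; On begin overlap it shows a widget and calls InteractLadder on the player, passing itself with CanClimb enabled.
; On end overlap it hides the widget, clears the player's CanClimb and returns movement to Walking.
; The widget toggles for any overlapping actor, as the player cast runs afterwards.
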(event OnComponentBeginOverlap(Box)
  (params (OverlappedComponent :type Primitive%20Component%20Object%20Reference) (OtherActor :type Actor%20Object%20Reference) (OtherComp :type Primitive%20Component%20Object%20Reference) (OtherBodyIndex :type Integer) (bFromSweep :type Boolean) (SweepResult :type Hit%20Result%20Structure%20%28by%20ref%29))
  (Rendering|SetVisibility (Variables|Default|GetWidget) true false)
  (bind _asbp_player (Utilities|Casting|CastToBP_Player OtherActor))
  (Default|InteractLadder _asbp_player self true))

(event OnComponentEndOverlap(Box)
  (params (OverlappedComponent :type Primitive%20Component%20Object%20Reference) (OtherActor :type Actor%20Object%20Reference) (OtherComp :type Primitive%20Component%20Object%20Reference) (OtherBodyIndex :type Integer))
  (Rendering|SetVisibility (Variables|Default|GetWidget) false false)
  (bind _asbp_player (Utilities|Casting|CastToBP_Player OtherActor))
  (Variables|/Game/player/BP_Player.BP_Player_C|SetcanClimb _asbp_player false)
  (Pawn|Components|CharacterMovement|SetMovementMode (Variables|/Script/Engine.Character|GetCharacterMovement _asbp_player) "MOVE_Walking" 0))

(fn ConstructionScript)