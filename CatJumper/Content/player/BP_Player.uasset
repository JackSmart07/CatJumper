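; BP_Player is the playable flipbook character, handling movement, jumping, NPC dialogue and ladder climbing.
; InteractNPC stores the speaker and current line, and Interact advances the dialogue line.
; Interact also sets Flying or Walking from CanClimb, which turns Move Up into vertical climbing, while InteractLadder is empty here.
; Tick picks idle, walk or jump flipbooks from velocity, and A/D keys rotate the sprite to face left or right.
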(event Custom|Interact%20Ladder
  (params (Ladder :type BP%20Ladder%20Object%20Reference) (CanClimb :type Boolean))
  ;[0.15 0.15 0.15 0.5] Called by BP_Ladder - Climb Ladder
)

(event Custom|Interact%20NPC
  (params (CanTalk :type Boolean) (NPCName :type String) (currentLine :type Integer))
  ;[0.15 0.15 0.15 0.5] Called by BP_NPC - Interacting w/ NPCS
  (Variables|Default|SetNPCName NPCName)
  (bind _output_get (Variables|Default|SetcurrentDialogueLine currentLine)))

(event EventTick
  (params (DeltaSeconds :type Float%20%28single-precision%29))
  (bind _fb_placeholder_idle (Variables|Default|GetFB_Placeholder_Idle))
  ;[0.15 0.15 0.15 0.5] Run cycle + jump animation
  (if (== (Math|Vector|VectorLength (Transformation|GetVelocity)) 0.0)
    (Sprite|SetFlipbook _fb_placeholder_idle "/Game/sprites/Placeholders/FB_Placeholder_Idle.FB_Placeholder_Idle" :!label _label)
    (elif (> (.z (Transformation|GetVelocity)) 0.0)
      (Sprite|SetFlipbook _fb_placeholder_idle "/Game/sprites/Placeholders/FB_Placeholder_Jump.FB_Placeholder_Jump")
      (elif (!= (.y (Transformation|GetVelocity)) 0.0) ; so branches are ordered\naccordingly
        (Sprite|SetFlipbook _fb_placeholder_idle "/Game/sprites/Placeholders/FB_Placeholder_Walk.FB_Placeholder_Walk")
        (else
          (goto _label))))))

(event Input|ActionEvents|InputActionInteract
  (params (Key :type Key%20Structure :default "None"))
  ;[0.15 0.15 0.15 0.5] Called by BP_NPC - Interacting w/ NPCS
  (:Pressed
    (Math|Integer|IncrementInt (stale Custom|Interact%20NPC _output_get))))

(event Input|ActionEvents|InputActionInteract
  (params (Key :type Key%20Structure :default "None"))
  (bind _charactermovement (Variables|Character|GetCharacterMovement))
  ;[0.15 0.15 0.15 0.5] Called by BP_Ladder - Climb Ladder
  (:Pressed
    (bind _output_get (Variables|Default|SetcanClimb (stale Custom|Interact%20Ladder CanClimb)))
    (if _output_get
      (Pawn|Components|CharacterMovement|SetMovementMode _charactermovement "MOVE_Flying" 0)
      (else
        (Pawn|Components|CharacterMovement|SetMovementMode _charactermovement "MOVE_Walking" 0)))))

(event Input|ActionEvents|InputActionJump
  (params (Key :type Key%20Structure :default "None"))
  ;[0.15 0.15 0.15 0.5] works for now. NOT sophisticated.
  (:Pressed
    (Character|Jump)))

(event Input|AxisEvents|InputAxisMoveUp
  (params (AxisValue :type Float%20%28single-precision%29))
  ;[0.15 0.15 0.15 0.5] Character movement modified from last game jam #IfItAintBrokeDontFixIt
  (if (Variables|Default|GetcanClimb)
    ;;[0.15 0.15 0.15 0.5] flying
    (Pawn|Input|AddMovementInput (Math|Vector|GetUpVector (Variables|Collision|GetCapsuleComponent)) AxisValue false) ; some help from https://youtu.be/ENux2q8sjoQ?si=K1_-qiRpIImei-wp
    (else
      (Pawn|Input|AddMovementInput (Math|Vector|GetForwardVector (Variables|Collision|GetCapsuleComponent)) AxisValue false))))

(event Input|AxisEvents|InputAxisMoveRight
  (params (AxisValue :type Float%20%28single-precision%29))
  ;[0.15 0.15 0.15 0.5] Character movement modified from last game jam #IfItAintBrokeDontFixIt
  (Pawn|Input|AddMovementInput (Math|Vector|GetRightVector (Variables|Collision|GetCapsuleComponent)) AxisValue false))

(event Input|KeyboardEvents|A
  (params (Key :type Key%20Structure :default "None"))
  ;[0.15 0.15 0.15 0.5] changing sprite 2 face left or right
  (:Pressed
    (if (not (Variables|Default|GetfacingLeft))
      (Transformation|AddLocalRotation (Variables|Default|GetFB_Placeholder_Idle) "0.000000,180.000000,0.000000" false false)
      (Variables|Default|SetfacingLeft true))))

(event Input|KeyboardEvents|D
  (params (Key :type Key%20Structure :default "None"))
  ;[0.15 0.15 0.15 0.5] changing sprite 2 face left or right
  (:Pressed
    (if (Variables|Default|GetfacingLeft)
      (Transformation|AddLocalRotation (Variables|Default|GetFB_Placeholder_Idle) "0.0,180.0,0.0" false false)
      (Variables|Default|SetfacingLeft false))))

(fn ConstructionScript)