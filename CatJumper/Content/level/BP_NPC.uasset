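; BP_NPC is an NPC Blueprint that shows a widget when something enters its Box trigger, intended for the player entering its radius.
; Begin overlap reveals the widget and prints NPCName to screen when it matches one of two hardcoded names, Des or Raven.
; End overlap hides the widget after a short delay, and neither event filters which actor overlapped.
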(event OnComponentBeginOverlap(Box)
  (params (OverlappedComponent :type Primitive%20Component%20Object%20Reference) (OtherActor :type Actor%20Object%20Reference) (OtherComp :type Primitive%20Component%20Object%20Reference) (OtherBodyIndex :type Integer) (bFromSweep :type Boolean) (SweepResult :type Hit%20Result%20Structure%20%28by%20ref%29))
  (bind _npcname (Variables|Default|GetNPCName))
  ;[0.15 0.15 0.15 0.5] player enters radius
  (Rendering|SetVisibility (Variables|Default|GetWidget) true false) ; https://www.youtube.com/watch?v=tob3GEdMJFc
  (if (Utilities|Enum|Equal(Enum) _npcname "Des")
    (Development|PrintString (Variables|Default|GetNPCName) :!label _label)
    (elif (Utilities|Enum|Equal(Enum) _npcname "Raven")
      (goto _label))))

(event OnComponentEndOverlap(Box)
  (params (OverlappedComponent :type Primitive%20Component%20Object%20Reference) (OtherActor :type Actor%20Object%20Reference) (OtherComp :type Primitive%20Component%20Object%20Reference) (OtherBodyIndex :type Integer))
  ;[0.15 0.15 0.15 0.5] player leaves radius
  (Utilities|FlowControl|Delay 0.8)
  (Rendering|SetVisibility (Variables|Default|GetWidget) false false))

(fn ConstructionScript)