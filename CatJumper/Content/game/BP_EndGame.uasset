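; BP_EndGame is the level's win trigger, ending the game when something overlaps its HitBox.
; An overlapping BP_Player has its movement mode set to None so it cannot slide away.
; A second sequence branch plays a sound, replaces all widgets with WG_GameWon and switches to UI-only input with a visible cursor.
; That branch sits outside the player cast, so any overlapping actor triggers the win screen.
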(event OnComponentBeginOverlap(HitBox)
  (params (OverlappedComponent :type Primitive%20Component%20Object%20Reference) (OtherActor :type Actor%20Object%20Reference) (OtherComp :type Primitive%20Component%20Object%20Reference) (OtherBodyIndex :type Integer) (bFromSweep :type Boolean) (SweepResult :type Hit%20Result%20Structure%20%28by%20ref%29))
  (bind _returnvalue (Game|GetPlayerController 0))
  (Utilities|FlowControl|Sequence
    (:then_0
      (bind _asbp_player (Utilities|Casting|CastToBP_Player OtherActor))
      (Pawn|Components|CharacterMovement|SetMovementMode (Variables|/Script/Engine.Character|GetCharacterMovement _asbp_player) "MOVE_None" 0) ; making sure player dont slide away
    )
    (:then_1
      ;[0.15 0.15 0.15 0.5] Plays endgame screen
      (Audio|PlaySound2D 0 1.0 1.0 0.0 0 0)
      (Viewport|RemoveAllWidgets)
      (bind _returnvalue_2 (UserInterface|CreateWidget "/Game/game/WG_GameWon.WG_GameWon_C"))
      (bind _output_get (Variables|Default|SetwinWidget _returnvalue_2))
      (UserInterface|Viewport|AddtoViewport _output_get 0)
      (Variables|/Script/Engine.PlayerController|SetbShowMouseCursor _returnvalue true)
      (Input|SetInputModeUIOnly _returnvalue _output_get "DoNotLock" false))))

(fn ConstructionScript)